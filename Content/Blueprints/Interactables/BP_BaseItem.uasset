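; Base interactable item that an instigator picks up into its inventory on interaction, described by an ItemInfo struct.
; Interaction checks space by item type: Catch Balls need trap space and stop any valid SFXToKill sound, while the other handled types need collectable space.
; On success it passes ItemInfo to the instigator's PickUpMessage and destroys itself.
; The construction script rebuilds ItemInfo to record the actor's own class.
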(event EventInteraction
  (params (Instigator :type Phase%20Player%20Character%20Object%20Reference))
  (bind _iteminfo (Variables|Default|GetItemInfo))
  (switch Utilities|FlowControl|Switch|SwitchonEItemTypes (.itemtype (Variables|Default|GetItemInfo))
    (:NewEnumerator1
      (if (Default|HasSpaceinCollectables Instigator) :!label _label
        (Class|Interact|PickUp(Message) Instigator (Variables|Default|GetItemInfo) :!label _label_2)
        (Actor|DestroyActor)))
    (:NewEnumerator2
      (goto _label))
    (:NewEnumerator3
      (goto _label))
    (:NewEnumerator4
      (goto _label))
    (:NewEnumerator6
      (goto _label))
    (:NewEnumerator7
      (if (Default|HasSpaceinTraps Instigator)
        (Utilities|IsValid (.sfxtokill (.trapinfo _iteminfo))
          (:Is%20Valid
            (Audio|Components|Audio|Stop (.sfxtokill (.trapinfo _iteminfo)))
            (goto _label_2))
          (:Is%20Not%20Valid
            (goto _label_2)))))))

(fn ConstructionScript
  (|CallParentFunction)
  (Variables|Default|SetItemInfo (Utilities|Struct|MakeFItemInfo (.itemtype (Variables|Default|GetItemInfo)) (.itemname (Variables|Default|GetItemInfo)) (.itemimage (Variables|Default|GetItemInfo)) (Utilities|GetClass self) (.itemindex (Variables|Default|GetItemInfo)) (.animalinfo (Variables|Default|GetItemInfo)) (.itemslot (Variables|Default|GetItemInfo)) (.itemvalue (Variables|Default|GetItemInfo)) (Utilities|Struct|MakeETrapItem (.traptype (.trapinfo (Variables|Default|GetItemInfo))) (.range (.trapinfo (Variables|Default|GetItemInfo))) (.attackspeed (.trapinfo (Variables|Default|GetItemInfo))) (.primarylefthandslot (.trapinfo (Variables|Default|GetItemInfo))) (.trapvfx (.trapinfo (Variables|Default|GetItemInfo))) (.trapsfx (.trapinfo (Variables|Default|GetItemInfo))) (.hitvfx (.trapinfo (Variables|Default|GetItemInfo))) (.hitsfx (.trapinfo (Variables|Default|GetItemInfo))) (.throwmontage (.trapinfo (Variables|Default|GetItemInfo))) 0))))