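; BP_baseInteractable is a base Blueprint for interactable objects in the game world.
; Its InteractableArea overlap events register and unregister the object with an overlapping PhasePlayerCharacter through interface-style messages.
; SetHighlight toggles custom depth rendering on InteractableMesh, and Interact is a default stub that returns false.
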(event OnComponentBeginOverlap(InteractableArea)
  (params (OverlappedComponent :type Primitive%20Component%20Object%20Reference) (OtherActor :type Actor%20Object%20Reference) (OtherComp :type Primitive%20Component%20Object%20Reference) (OtherBodyIndex :type Integer) (bFromSweep :type Boolean) (SweepResult :type Hit%20Result%20Structure%20%28by%20ref%29))
  (bind _asphase_player_character (Utilities|Casting|CastToPhasePlayerCharacter OtherActor))
  (Class|Interact|RegisterInteractable(Message) _asphase_player_character self))

(event OnComponentEndOverlap(InteractableArea)
  (params (OverlappedComponent :type Primitive%20Component%20Object%20Reference) (OtherActor :type Actor%20Object%20Reference) (OtherComp :type Primitive%20Component%20Object%20Reference) (OtherBodyIndex :type Integer))
  (bind _asphase_player_character (Utilities|Casting|CastToPhasePlayerCharacter OtherActor))
  (Class|Interact|UnregisterInteractable(Message) _asphase_player_character self))

(fn ConstructionScript)

(fn SetHighlight
  (params (Highlight? :type Boolean))
  (Rendering|SetRenderCustomDepth (Variables|Default|GetInteractableMesh) Highlight?))

(fn Interact
  (params (Actor :type Actor%20Object%20Reference) (TargetPoint :type Scene%20Component%20Object%20Reference))
  (return false))